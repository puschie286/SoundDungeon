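; Cube actor that stretches along a selectable axis to visualise a live value read from a shared data slot.
; BeginPlay stores the start location and builds a scaling from configured value and scale ranges.
; Tick, throttled by a Delay, maps the slot value to scale, subtracts ReduceSize and applies it.
; CalculateLocation shifts the actor by half its size to grow one way, but only ever offsets along Y.
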(event EventTick
  (params (DeltaSeconds :type Float%20%28single-precision%29))
  (Utilities|FlowControl|Delay (Variables|Default|GetUpdateIntervall))
  (bind _storeddata (Class|WAVLibrary|LIBGetShare (Variables|Default|GetUseSlot)))
  (bind _scaledvalue (Class|WAVLibrary|LIBScaleGetScaled (Variables|Default|GetScaleY) (Utilities|Array|Get(acopy) _storeddata (Variables|Default|GetUseDataSlot))))
  (switch string (Variables|Default|GetScale)
    (:Default
      (Transformation|SetWorldScale3D (Math|Vector|MakeVector 1.0 (- _scaledvalue (Variables|Default|GetReduceSize)) 1.0) :!label _label))
    (:-Y
      (goto _label))
    (:Y
      (goto _label))
    (:-Z
      (Transformation|SetWorldScale3D (Math|Vector|MakeVector 1.0 1.0 (- _scaledvalue (Variables|Default|GetReduceSize))) :!label _label_2))
    (:Z
      (goto _label_2))
    (:-X
      (Transformation|SetWorldScale3D (Math|Vector|MakeVector (- _scaledvalue (Variables|Default|GetReduceSize)) 1.0 1.0) :!label _label_3))
    (:X
      (goto _label_3)))
  (bind _newlocation (CallFunction|CalculateLocation (- _scaledvalue (Variables|Default|GetReduceSize))))
  (Transformation|SetActorLocation _newlocation false))

(event EventBeginPlay
  (Variables|Default|SetDefaultPosition (Transformation|GetActorLocation))
  (Variables|Default|SetScaleY (Utilities|Struct|MakeScaling -1e+02 1e+02 (Variables|Default|GetMinScale) (Variables|Default|GetMaxScale) (Variables|Default|GetCurMin) (Variables|Default|GetCurMax) false true (Variables|Default|GetInterpolateIntervall))))

(fn ConstructionScript)

(fn CalculateLocation
  (params (ScaledValue :type Float%20%28single-precision%29))
  (bind _returnvalue (/ ScaledValue 2.0))
  (bind _defaultposition (Variables|Default|GetDefaultPosition))
  (bind (_x _y _z) (Math|Vector|BreakVector _defaultposition))
  (bind _returnvalue_2 (* _returnvalue 1e+02))
  (switch string (Variables|Default|GetScale)
    (:Default
      (Variables|Default|SetTempLocation (Math|Vector|MakeVector _x (- _y _returnvalue_2) _z) :!label _label))
    (:-Y
      (goto _label))
    (:Y
      (bind _output_get (Variables|Default|SetTempLocation (Math|Vector|MakeVector _x (+ _returnvalue_2 _y) _z)))))
  (return _output_get))