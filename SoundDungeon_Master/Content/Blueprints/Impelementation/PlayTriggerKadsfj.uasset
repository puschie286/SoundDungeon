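; Trigger actor that plays two sound sources while the player overlaps it and starts a Matinee once both pass a time check.
; Begin overlap stores the ExamplePlayerCharacter and starts both sounds; end overlap clears it and stops them.
; Tick, throttled by a half-second Delay, polls TimeCheck on each source while the player reference is valid.
; When both return true, it plays the Matinee and disables its own tick.
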(event EventActorBeginOverlap
  (params (OtherActor :type Actor%20Object%20Reference))
  (bind _asexample_player_character (Utilities|Casting|CastToExamplePlayerCharacter OtherActor))
  (Variables|Default|SetPlayerRef _asexample_player_character)
  (Default|PlayAudio (Variables|Default|GetSoundSource)))

(event EventActorEndOverlap
  (params (OtherActor :type Actor%20Object%20Reference))
  (Utilities|Casting|CastToExamplePlayerCharacter OtherActor)
  (Variables|Default|SetPlayerRef 0)
  (Class|SoundSource|StopSound (Variables|Default|GetSoundSource)))

(event EventTick
  (params (DeltaSeconds :type Float%20%28single-precision%29))
  (Utilities|FlowControl|Delay 0.5)
  (Utilities|IsValid (Variables|Default|GetPlayerRef)
    (:Is%20Valid
      (bind _check (Default|TimeCheck (Variables|Default|GetSoundSource)))
      (if _check
        (bind _check_2 (Default|TimeCheck (Variables|Default|GetSoundSource1)))
        (if _check_2
          (Audio|Components|Audio|Play (Variables|Default|GetMatinee))
          (Actor|Tick|SetActorTickEnabled false))))))

(fn ConstructionScript)