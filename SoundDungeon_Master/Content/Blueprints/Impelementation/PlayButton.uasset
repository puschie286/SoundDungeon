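; PlayButton is an interactable button that plays three sound sources and checks whether all of them pass a timing check, apparently as an audio puzzle.
; Its Action function starts audio on every source, then runs TimeCheck on each in a nested chain.
; When all three checks succeed it plays a Matinee sequence, and the function returns the check result.
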(fn ConstructionScript)

(fn Action
  (params (Target :type Actor%20Object%20Reference))
  (bind _soundsource (Variables|Default|GetSoundSource))
  (bind _soundsource1 (Variables|Default|GetSoundSource1))
  (bind _soundsource2 (Variables|Default|GetSoundSource2))
  (Utilities|FlowControl|Sequence
    (:then_0
      (Default|PlayAudio _soundsource)
      (Default|PlayAudio _soundsource1)
      (Default|PlayAudio _soundsource2))
    (:then_1
      (bind _check (Default|TimeCheck _soundsource))
      (if _check
        (bind _check_2 (Default|TimeCheck _soundsource1))
        (if _check_2
          (bind _check_3 (Default|TimeCheck _soundsource2))
          (bind _output_get (LocalVariables|SetbResult _check_3))
          (if _output_get
            (Audio|Components|Audio|Play (Variables|Default|GetMatinee)))))
      (return _output_get))))