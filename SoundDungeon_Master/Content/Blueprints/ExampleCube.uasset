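; Example audio-visualizer actor that loads a WAV file, generates a waveform mesh and drives a light and component rotation from the music.
; While audio plays, delayed Tick updates multiply short-window amplitude buckets by a frequency spectrum at the current play time.
; The first band of that result is remapped through per-effect scales to set light intensity and pitch.
; An optional debug flag prints each normalized scaled value.
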(event EventTick
  (params (DeltaSeconds :type Float%20%28single-precision%29))
  (bind _wav_data (Variables|Default|GetWAV%20Data))
  (bind _extendedaudio (Variables|Default|GetExtendedAudio))
  (bind _playtime (Variables|/Script/SoundDungeon_Master.ExtendedAudioComponent|GetPlayTime _extendedaudio))
  ;[1 1 1] Event while Music Playing in Intervals
  (bind _returnvalue (Audio|Components|Audio|IsPlaying _extendedaudio))
  (if _returnvalue
    (Utilities|FlowControl|Delay 0.02)
    (Utilities|FlowControl|Sequence
      (:then_0
        ;[1 1 1] Calculate Data & Save
        (bind _outamplitudes (Class|WAVLibrary|LIBGetAmplitude 0 _playtime 0.02 5 _wav_data)))
      (:then_1
        (bind _outspectrum (Class|WAVLibrary|LIBCalculateFrequencySpectrum 0 _playtime 0.02 5 _wav_data))
        (bind _resultarray (Class|WAVLibrary|LIBArrayMultiply _outamplitudes _outspectrum))
        (Variables|Default|SetCalculated%20Data _resultarray))
      (:then_2
        ;[1 1 1] Example Functions
        (CallFunction|SCALED-LightIntensity)
        (CallFunction|SCALED-ActorRotation)))))

(event EventBeginPlay
  ;[1 1 1] Init Audio File
  (bind _outdata (Class|WAVLibrary|LIBGetWAV (Variables|Default|GetWavFile%20Name) true))
  (Variables|Default|SetWAV%20Data _outdata)
  ;[1 1 1] Generate Waveform-Mesh
  (Class|WAVLibrary|LIBGenerateWaveform (Variables|Default|GetWAV%20Data) (Variables|Default|GetCustomMesh) false false 300 100))

(fn ConstructionScript)

(fn SCALED-LightIntensity
  (params (Array%20Slot :type Integer :default 0))
  (bind _scaledvalue (Class|WAVLibrary|LIBScaleGetScaled (Variables|Default|GetLight%20Intensity%20Scale) (Utilities|Array|Get(acopy) (Variables|Default|GetCalculated%20Data) Array%20Slot)))
  (Rendering|Components|Light|SetIntensity (Variables|Default|GetExample%20Scaled%20Intensity) _scaledvalue)
  ;[1 1 1] Debug
  (if (Variables|Default|GetDebugActive)
    (CallFunction|DebugScale (Variables|Default|GetLight%20Intensity%20Scale) _scaledvalue "Actor :")))

(fn SCALED-ActorRotation
  (params (Array%20Slot :type Integer :default 0))
  (bind _example_scaled_rotation (Variables|Default|GetExample%20Scaled%20Rotation))
  (bind _relativerotation (Variables|/Script/Engine.SceneComponent|GetRelativeRotation _example_scaled_rotation))
  (bind (_pitch _yaw _roll) (Class|KismetMathLibrary|BreakRot _relativerotation))
  (bind _scaledvalue (Class|WAVLibrary|LIBScaleGetScaled (Variables|Default|GetActor%20Rotation%20Scale) (Utilities|Array|Get(acopy) (Variables|Default|GetCalculated%20Data) Array%20Slot)))
  (Transformation|SetRelativeRotation (Variables|Default|GetExample%20Scaled%20Rotation) (Class|KismetMathLibrary|MakeRot _scaledvalue _yaw _roll) false)
  ;[1 1 1] Debug
  (if (Variables|Default|GetDebugActive)
    (CallFunction|DebugScale (Variables|Default|GetActor%20Rotation%20Scale) _scaledvalue "Actor :")))

(fn DebugScale
  (params (Scale :type Scaling%20Structure) (ScaledValue :type Float%20%28single-precision%29 :default 0.0) (Prefix :type String))
  (bind (_minvalue _maxvalue _minscale _maxscale) (Utilities|Struct|BreakScaling Scale))
  (bind _returnvalue (- 0.0 _minscale))
  (Development|PrintString (Utilities|String|BuildString(Float) "" Prefix (/ (+ ScaledValue _returnvalue) (+ _returnvalue _maxscale)))))