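; TestLight is a spot light actor for the sound visualization test room whose intensity follows a value from shared library data.
; On Tick, a short Delay throttles updates, then it fetches the array for its share slot and picks one data index.
; It scales that value through a library function and sets the light intensity, switching to zero below a minimum threshold.
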(event EventTick
  (params (DeltaSeconds :type Float%20%28single-precision%29))
  (bind _spotlightcomponent (Variables|Default|GetSpotLightComponent))
  (Utilities|FlowControl|Delay 0.05)
  (bind _storeddata (Class|WAVLibrary|LIBGetShare (Variables|Default|GetUseSlot)))
  (bind _scaledvalue (Class|WAVLibrary|LIBScaleGetScaled (Variables|Default|GetLightScaling) (Utilities|Array|Get(acopy) _storeddata (Variables|Default|GetUseDataSlot))))
  (if (< _scaledvalue (Variables|Default|GetMinIntensity))
    (Rendering|Components|Light|SetIntensity _spotlightcomponent 0.0)
    (else
      (Rendering|Components|Light|SetIntensity _spotlightcomponent _scaledvalue))))

(fn ConstructionScript)