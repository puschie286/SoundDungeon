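; An example Blueprint for audio visualization that exercises WAV waveform and playback analysis functions.
; On BeginPlay it calls LoadData, prints part of the "MainVocal" WAV data and passes CustomMesh to LIBGetWaveform for that WAV.
; Each Tick samples bucketed amplitude and frequency spectrum over a short window at VisualizableAudio's play time.
; Their combined value only feeds a PrintString with screen and log output disabled.
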(event EventBeginPlay
  (Class|VisualizableAudioComponent|LoadData "None")
  (bind _outdata (Class|WAVLibrary|LIBGetWAV "MainVocal"))
  (Development|PrintString (Utilities|String|ToString(Byte) (Utilities|Array|Get(acopy) _outdata)))
  (Class|WAVLibrary|LIBGetWaveform "MainVocal" (Variables|Default|GetCustomMesh)))

(event EventTick
  (params (DeltaSeconds :type Float%20%28single-precision%29))
  (bind _visualizableaudio (Variables|Default|GetVisualizableAudio))
  (bind _playtime (Variables|/Script/SoundDungeon_Master.VisualizableAudioComponent|GetPlayTime _visualizableaudio))
  (Utilities|FlowControl|Sequence
    (:then_0
      (bind _outamplitudes (Class|VisualizableAudioComponent|GetAmplitude 0 _playtime 0.01 10))
      (bind _outspectrum (Class|VisualizableAudioComponent|CalculateFrequencySpectrum 0 _playtime 0.01 10))
      (Development|PrintString (Utilities|String|ToString(Float) (Math|Float|%(Float) (* (Utilities|Array|Get(acopy) _outamplitudes 5) (Utilities|Array|Get(acopy) _outspectrum 5)) 5e+02)) false false))))

(fn ConstructionScript)