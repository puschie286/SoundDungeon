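; Test point light for the sound visualization test room that drives its intensity from shared data.
; Tick runs through a short Delay, then reads one data slot of the selected share slot via LIBGetShare and scales it with LightScaling.
; The scaled value sets the PointLightComponent intensity, or zero when it falls below MinIntensity.
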(event EventTick
  (params (DeltaSeconds :type Float%20%28single-precision%29))
  (bind _pointlightcomponent (Variables|Default|GetPointLightComponent))
  (Utilities|FlowControl|Delay 0.05)
  (bind _storeddata (Class|WAVLibrary|LIBGetShare (Variables|Default|GetUseSlot)))
  (bind _scaledvalue (Class|WAVLibrary|LIBScaleGetScaled (Variables|Default|GetLightScaling) (Utilities|Array|Get(acopy) _storeddata (Variables|Default|GetUseDataSlot))))
  (if (< _scaledvalue (Variables|Default|GetMinIntensity))
    (Rendering|Components|Light|SetIntensity _pointlightcomponent 0.0)
    (else
      (Rendering|Components|Light|SetIntensity _pointlightcomponent _scaledvalue))))

(fn ConstructionScript)