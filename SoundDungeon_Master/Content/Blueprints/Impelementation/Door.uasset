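; Sliding double-door Blueprint that opens when something overlaps either of its two trigger volumes.
; BeginPlay caches start and end positions for both leaves, offset by Distance in opposite Y directions, with an extra fixed Y shift on the right start.
; Both triggers play one timeline that lerps the leaves' relative locations apart.
; The graph has no closing logic or filter on the overlapping actor.
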(event OnComponentBeginOverlap(Trigger1)
  (params (OtherActor :type Actor%20Object%20Reference) (OtherComp :type Primitive%20Component%20Object%20Reference) (OtherBodyIndex :type Integer) (bFromSweep :type Boolean) (SweepResult :type Hit%20Result%20Structure%20%28by%20ref%29))
  (bind _driver (Timeline|Timeline_DoorFrame Play)
    (:Update
      (Transformation|SetRelativeLocation (Variables|Default|GetLeftDoor) (Math|Vector|Lerp(Vector) (Variables|Default|GetDoorLeftStart) (Variables|Default|GetDoorLeftEnd) _driver) false)
      (Transformation|SetRelativeLocation (Variables|Default|GetRightDoor) (Math|Vector|Lerp(Vector) (Variables|Default|GetDoorRightStart) (Variables|Default|GetDoorRightEnd) _driver) false))))

(event OnComponentBeginOverlap(Trigger0)
  (params (OtherActor :type Actor%20Object%20Reference) (OtherComp :type Primitive%20Component%20Object%20Reference) (OtherBodyIndex :type Integer) (bFromSweep :type Boolean) (SweepResult :type Hit%20Result%20Structure%20%28by%20ref%29))
  (bind _driver (Timeline|Timeline_DoorFrame Play)
    (:Update
      (Transformation|SetRelativeLocation (Variables|Default|GetLeftDoor) (Math|Vector|Lerp(Vector) (Variables|Default|GetDoorLeftStart) (Variables|Default|GetDoorLeftEnd) _driver) false)
      (Transformation|SetRelativeLocation (Variables|Default|GetRightDoor) (Math|Vector|Lerp(Vector) (Variables|Default|GetDoorRightStart) (Variables|Default|GetDoorRightEnd) _driver) false))))

(event EventBeginPlay
  (bind _distance (Variables|Default|GetDistance))
  (bind _returnvalue (Math|Vector|MakeVector 0.0 _distance 0.0))
  (Utilities|FlowControl|Sequence
    (:then_0
      (bind _output_get (Variables|Default|SetDoorLeftStart (Variables|/Script/Engine.SceneComponent|GetRelativeLocation (Variables|Default|GetLeftDoor))))
      (Variables|Default|SetDoorLeftEnd (+ _output_get _returnvalue)))
    (:then_1
      (bind _output_get_2 (Variables|Default|SetDoorRightStart (+ (Variables|/Script/Engine.SceneComponent|GetRelativeLocation (Variables|Default|GetDoorRight)) "0,-150.000000, 0")))
      (Variables|Default|SetDoorRightEnd (- _output_get_2 _returnvalue)))))

(fn ConstructionScript)