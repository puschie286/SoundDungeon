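; MusicBox is an actor that varies the volume of its audio component by the player's distance from it.
; A Box overlap stores the ExamplePlayerCharacter reference, then clears it and resets the volume to a fixed multiplier on exit.
; While the reference is valid, Tick passes the distance through a scale library function using the Scale variable to set the volume multiplier.
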(event OnComponentBeginOverlap(Box)
  (params (OtherActor :type Actor%20Object%20Reference) (OtherComp :type Primitive%20Component%20Object%20Reference) (OtherBodyIndex :type Integer) (bFromSweep :type Boolean) (SweepResult :type Hit%20Result%20Structure%20%28by%20ref%29))
  (bind _asexample_player_character (Utilities|Casting|CastToExamplePlayerCharacter OtherActor))
  (Variables|Default|SetPlayerRef _asexample_player_character))

(event OnComponentEndOverlap(Box)
  (params (OtherActor :type Actor%20Object%20Reference) (OtherComp :type Primitive%20Component%20Object%20Reference) (OtherBodyIndex :type Integer))
  (Utilities|Casting|CastToExamplePlayerCharacter OtherActor)
  (Variables|Default|SetPlayerRef 0)
  (Audio|Components|Audio|SetVolumeMultiplier (Variables|Default|GetAudio) 0.3 :!class /Script/Engine.AudioComponent))

(event EventTick
  (params (DeltaSeconds :type Float%20%28single-precision%29))
  (Utilities|IsValid (Variables|Default|GetPlayerRef)
    (:Is%20Valid
      (bind _scaledvalue (Class|WAVLibrary|LIBScaleGetScaled (Variables|Default|GetScale) (Math|Vector|VectorLength (- (Transformation|GetActorLocation) (Transformation|GetActorLocation (Variables|Default|GetPlayerRef))))))
      (Audio|Components|Audio|SetVolumeMultiplier (Variables|Default|GetAudio) _scaledvalue :!class /Script/Engine.AudioComponent))))

(fn ConstructionScript)