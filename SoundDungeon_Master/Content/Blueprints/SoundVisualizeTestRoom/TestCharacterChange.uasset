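; Trigger actor in the sound visualization test room that switches the player to an ExampleTubePlayer on overlap.
; Any actor overlap spawns the tube player at a valid SpawnPoint, removes an existing ExamplePlayerCharacter and its HUD, then possesses the new pawn.
; The tube player's Radius comes from the floored relative Z of the SpawnPoint's first camera component.
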(event EventActorBeginOverlap
  (params (OtherActor :type Actor%20Object%20Reference))
  (bind _spawnpoint (Variables|Default|GetSpawnPoint))
  (Utilities|IsValid _spawnpoint
    (:Is%20Valid
      (bind _returnvalue (Game|SpawnActorfromClass "/Game/Blueprints/Examples/ExampleTubePlayer.ExampleTubePlayer_C" (Transformation|GetActorTransform _spawnpoint) false 0))
      (CallFunction|RemoveOldPlayer)
      (Pawn|Possess (Game|GetPlayerController 0) _returnvalue)
      (CallFunction|SetRadius _returnvalue))))

(fn ConstructionScript)

(fn SetRadius
  (params (TubePlayer :type Tube%20Player%20Object%20Reference))
  (Variables|/Script/SoundDungeon_Master.TubePlayer|SetRadius TubePlayer (Math|Float|Floor (.Z (Math|Vector|BreakVector (Variables|/Script/Engine.SceneComponent|GetRelativeLocation (Utilities|Array|Get(acopy) (Actor|GetComponentsByClass (Variables|Default|GetSpawnPoint) "/Script/Engine.CameraComponent")))))))
  (return))

(fn RemoveOldPlayer
  (bind _returnvalue (Game|GetPlayerCharacter 0))
  (bind _asexample_player_character (Utilities|Casting|CastToExamplePlayerCharacter _returnvalue)
    (:then
      (Widget|RemovefromParent (Variables|/Game/Blueprints/Examples/ExamplePlayerCharacter.ExamplePlayerCharacter_C|GetHUDRef _asexample_player_character))
      (Actor|DestroyActor _returnvalue))
    (:CastFailed
      _))
  (return))