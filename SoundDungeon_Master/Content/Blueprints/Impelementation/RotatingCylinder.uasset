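; Rotating cylinder actor that turns once around its yaw axis when triggered, locking player input during the motion.
; Calling Rotating derives a yaw speed from RotationRange and RotationTime and starts the countdown.
; Tick applies the incremental rotation, disables player character input once at the start, and re-enables it once time runs out.
; Neither state flag is reset, so the rotation runs only once.
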(event EventTick
  (params (DeltaSeconds :type Float%20%28single-precision%29))
  (if (Variables|Default|GetRotationFInish)
    (Utilities|FlowControl|DoOnce false
      (:Completed
        (Input|EnableInput (Game|GetPlayerCharacter 0) 0)))
    (elif (Variables|Default|GetOnRotation)
      (Utilities|FlowControl|Sequence
        (:then_0
          (bind _output_get (Variables|Default|SetRotation (Class|KismetMathLibrary|MakeRot (.Pitch (Class|KismetMathLibrary|BreakRot (Variables|Default|GetRotation))) (+ (* DeltaSeconds (Variables|Default|GetStep)) (.Yaw (Class|KismetMathLibrary|BreakRot (Variables|Default|GetRotation)))) (.Roll (Class|KismetMathLibrary|BreakRot (Variables|Default|GetRotation))))))
          (Transformation|SetActorRelativeRotation _output_get)
          (bind _output_get_2 (Variables|Default|SetTime (- (Variables|Default|GetTime) DeltaSeconds)))
          (if (< _output_get_2 0.0)
            (Variables|Default|SetRotationFInish true)))
        (:then_1
          (Utilities|FlowControl|DoOnce false
            (:Completed
              (Input|DisableInput (Game|GetPlayerCharacter 0) 0))))))))

(event EventBeginPlay
  (Variables|Default|SetRotation (Transformation|GetActorRotation)))

(fn ConstructionScript)

(fn Rotating
  (if (not (Variables|Default|GetOnRotation))
    (bind _output_get (Variables|Default|SetTime (Variables|Default|GetRotationTime)))
    (Variables|Default|SetStep (/ (Variables|Default|GetRotationRange) _output_get))
    (Variables|Default|SetOnRotation true)))