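; TestTube is a sound visualization test Blueprint that generates a tube from a named WAV file's data.
; On BeginPlay it force-fetches the WAV via LIBGetWAV and passes it to LIBGenerateTube with a Width/Height waveform config, using itself as the base cube.
; A copy of the same logic sits disconnected in the Construction Script, so generation happens only at runtime.
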(event EventBeginPlay
  (bind _outdata (Class|WAVLibrary|LIBGetWAV (Variables|Default|GetWAV%20Name) true))
  (Class|WAVLibrary|LIBGenerateTube _outdata (Utilities|Struct|MakeWaveformConfig 0 false false false (Variables|Default|GetWidth) (Variables|Default|GetHeight)) self))

(fn ConstructionScript)